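; Procedural tunnel terrain segment that has noise-driven holes and flashes to the music beat.
; Construction script appends boxes in a ring around the X axis using Geometry Script, with width derived from radius and side count.
; It boolean-subtracts hole boxes chosen by noise from world position and MusicData, then generates convex-hull collision.
; On BeginPlay it binds to BP_MusicPlayer's beat dispatcher to briefly pulse FlashOn on a dynamic material.
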(event Custom|Setup%20Material
  (bind _dynamic_mesh_component (Variables|Default|GetDynamic%20Mesh%20Component))
  (bind _returnvalue (Rendering|Material|CreateDynamicMaterialInstance _dynamic_mesh_component 0 "/Game/Materials/M_MusicResponse.M_MusicResponse" "None" :!class /Script/Engine.PrimitiveComponent))
  (bind _returnvalue_2 (Actor|GetActorOfClass "/Game/LevelActors/BP_MusicPlayer.BP_MusicPlayer_C"))
  (Rendering|Material|SetMaterial _dynamic_mesh_component 0 _returnvalue)
  (EventDispatchers|BindEventtoBeatCompleteDispatcher _returnvalue_2 (delegate Custom|On%20Beat%20Completed)))

(event Custom|On%20Beat%20Completed
  (Rendering|Material|SetScalarParameterValue (stale Custom|Setup%20Material _returnvalue) "FlashOn" 1.0 :!class /Script/Engine.MaterialInstanceDynamic)
  (Utilities|FlowControl|Delay 0.1)
  (Rendering|Material|SetScalarParameterValue (stale Custom|Setup%20Material _returnvalue) "FlashOn" 0.0 :!class /Script/Engine.MaterialInstanceDynamic))

(event EventBeginPlay
  (CallFunction|SetupMaterial))

(fn ConstructionScript
  (bind _radius (Variables|Default|GetRadius))
  (Variables|Default|SetWidth (* (Variables|Default|GetRadius) 2.0 (Math|Trig|Sin(Radians) (/ (Math|Trig|GetPI) (Variables|Default|GetNumber%20of%20Sides)))))
  (bind _returnvalue (DynamicMeshComponent|GetDynamicMesh (Variables|Default|GetDynamic%20Mesh%20Component)))
  (bind _output_get (Variables|Default|SetDynamic%20Mesh _returnvalue))
  (for _index (range 0 (- (Variables|Default|GetNumber%20of%20Sides) 1))
    (Utilities|Array|Add (Variables|Default|GetBox%20Locations) (Math|Transform|MakeTransform (Math|Vector|MakeVector 0.0 (* (Math|Trig|Sin(Radians) (Math|Trig|DegreesToRadians (* _index (/ (Math|Float|MakeLiteralFloat 3.6e+02) (Variables|Default|GetNumber%20of%20Sides))))) _radius) (* (Math|Trig|Cos(Radians) (Math|Trig|DegreesToRadians (* _index (/ (Math|Float|MakeLiteralFloat 3.6e+02) (Variables|Default|GetNumber%20of%20Sides))))) _radius)) (Math|Rotator|MakeRotator (+ (* _index (/ (Math|Float|MakeLiteralFloat 3.6e+02) (Variables|Default|GetNumber%20of%20Sides))) 1.8e+02) 0.0 0.0)))
    (Class|GeometryScriptLibraryMeshPrimitiveFunctions|AppendBox :TargetMesh _output_get :Transform (Math|Transform|MakeTransform (Math|Vector|MakeVector 0.0 (* (Math|Trig|Sin(Radians) (Math|Trig|DegreesToRadians (* _index (/ (Math|Float|MakeLiteralFloat 3.6e+02) (Variables|Default|GetNumber%20of%20Sides))))) _radius) (* (Math|Trig|Cos(Radians) (Math|Trig|DegreesToRadians (* _index (/ (Math|Float|MakeLiteralFloat 3.6e+02) (Variables|Default|GetNumber%20of%20Sides))))) _radius)) (Math|Rotator|MakeRotator (+ (* _index (/ (Math|Float|MakeLiteralFloat 3.6e+02) (Variables|Default|GetNumber%20of%20Sides))) 1.8e+02) 0.0 0.0)) :DimensionX (Variables|Default|GetLength) :DimensionY (Variables|Default|GetWidth) :DimensionZ 2e+01 :Debug 0))
  (CallFunction|SetupBooleanMesh)
  (GeometryScript|Booleans|ApplyMeshBoolean :TargetMesh (Variables|Default|GetDynamic%20Mesh) :ToolMesh (Variables|Default|GetBoolean%20Mesh) :Operation "Subtract" :Debug 0)
  (bind _returnvalue_2 (Class|GeometryScriptLibraryCollisionFunctions|GenerateCollisionfromMesh (Variables|Default|GetDynamic%20Mesh) (Utilities|Struct|MakeGeometryScriptCollisionfromMeshOptions true "ConvexHulls" true true true 1.0 false 25 25) 0))
  (Class|GeometryScriptLibraryCollisionFunctions|SetSimpleCollisionOfDynamicMeshComponent :SimpleCollision _returnvalue_2 :DynamicMeshComponent (Variables|Default|GetDynamic%20Mesh%20Component) :Debug 0)
  (bind _returnvalue_3 (DynamicMeshComponent|GetDynamicMesh (Variables|Default|GetBoolean%20Mesh%20Component)))
  (DynamicMesh|Reset _returnvalue_3))

(fn SetupBooleanMesh
  (bind _returnvalue (DynamicMeshComponent|GetDynamicMesh (Variables|Default|GetBoolean%20Mesh%20Component)))
  (Variables|Default|SetBoolean%20Mesh _returnvalue)
  (for _array_element (Variables|Default|GetBox%20Locations)
    (bind _returnvalue_2 (Class|AnalyzerFunctionLibrary|CalculateNoiseResults (+ (.Location (Math|Transform|BreakTransform _array_element)) (Transformation|GetActorLocation)) (Variables|Default|GetMusic%20Data)))
    (if (.isHole (Utilities|Struct|BreakNoiseResultData _returnvalue_2))
      (Class|GeometryScriptLibraryMeshPrimitiveFunctions|AppendBox :TargetMesh (Variables|Default|GetBoolean%20Mesh) :Transform (Math|Transform|MakeTransform (+ (.transformOffset (Utilities|Struct|BreakNoiseResultData _returnvalue_2)) (.Location (Math|Transform|BreakTransform _array_element))) (.Rotation (Math|Transform|BreakTransform _array_element)) (.Scale (Math|Transform|BreakTransform _array_element))) :DimensionX (.sizeX (Utilities|Struct|BreakNoiseResultData _returnvalue_2)) :DimensionY (.sizeY (Utilities|Struct|BreakNoiseResultData _returnvalue_2)) :Debug 0))))