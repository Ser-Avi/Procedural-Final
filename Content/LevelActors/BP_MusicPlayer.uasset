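; Level actor that plays the song named in the game instance and broadcasts its beats during play.
; On BeginPlay it fetches that song's music data and, if the BPM is non-zero, initializes BP_TerrainManager with it, starts the beat loop and spawns the 2D sound.
; HandleBeats re-calls itself after each precomputed beat-gap delay, firing a beat-complete dispatcher.
; Song end only prints a message, via a timer event and delay.
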(event Custom|Handle%20Beats
  (Utilities|FlowControl|Delay (Utilities|Array|Get(acopy) (.beats_diff (Utilities|Struct|BreakMusicData (Variables|Default|GetMusic%20Data))) (Variables|Default|GetBeats%20Elapsed)))
  (Math|Integer|IncrementInt (Variables|Default|GetBeats%20Elapsed)
    (:%20%20
      (Default|CallBeatCompleteDispatcher)
      (CallFunction|HandleBeats))))

(event Custom|Initialize
  (bind _asbp_third_person_game_instance (Utilities|Casting|CastToBP_ThirdPersonGameInstance (Game|GetGameInstance)))
  (bind _returnvalue (Class|AnalyzerFunctionLibrary|GetData (Variables|/Game/ThirdPerson/Blueprints/BP_ThirdPersonGameInstance.BP_ThirdPersonGameInstance_C|GetSong%20Name _asbp_third_person_game_instance)))
  (bind _output_get (Variables|Default|SetMusic%20Data _returnvalue))
  (bind _output_get_2 (Variables|Default|SetData%20Loaded%20Properly (!= (.bpm (Utilities|Struct|BreakMusicData _output_get)) 0.0)))
  (if _output_get_2
    (bind _returnvalue_2 (Actor|GetActorOfClass "/Game/LevelActors/BP_TerrainManager.BP_TerrainManager_C"))
    (Default|Initialize _returnvalue_2 (Variables|Default|GetMusic%20Data))
    (CallFunction|HandleBeats)
    (bind _returnvalue_3 (Audio|SpawnSound2D (.sound (Utilities|Struct|BreakMusicData _output_get)) 1.0 1.0 0.0 0))
    (bind _output_get_3 (Variables|Default|SetAudio%20Component _returnvalue_3))
    (bind _returnvalue_4 (Animation|GetPlayLength _output_get_3))
    (Utilities|Time|SetTimerbyEvent (delegate Custom|On%20Song%20Finished) 0.0)
    (else
      (Development|PrintString "Failed to Load Song Info"))))

(event Custom|On%20Song%20Finished
  (Utilities|FlowControl|Delay (stale Custom|Initialize _returnvalue_4))
  (Development|PrintString "Song Finished"))

(event EventBeginPlay
  (bind _asbp_third_person_game_instance (Utilities|Casting|CastToBP_ThirdPersonGameInstance (Game|GetGameInstance)))
  (Variables|Default|SetSong%20Name (Variables|/Game/ThirdPerson/Blueprints/BP_ThirdPersonGameInstance.BP_ThirdPersonGameInstance_C|GetSong%20Name _asbp_third_person_game_instance))
  (CallFunction|Initialize))

(fn ConstructionScript)